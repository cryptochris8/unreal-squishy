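; BP_SquishyCharacter is the player character that squishes BP_SquishyFriend actors in front of it.
; On BeginPlay it adds the IMC_Squishy Enhanced Input mapping context to the first player controller.
; The IA_Squish action fires a short forward line trace on the Visibility channel, offset below the actor's location, and calls Squish on any BP_SquishyFriend it hits.
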(event Input|EnhancedActionEvents|EnhancedInputActionIA_Squish
  (params (ActionValue :type Boolean) (ElapsedSeconds :type Float%20%28double-precision%29) (TriggeredSeconds :type Float%20%28double-precision%29) (InputAction :type Input%20Action%20Object%20Reference :default "/Game/SquishySmash/Input/IA_Squish.IA_Squish"))
  (CallFunction|OnSquishPressed))

(event EventBeginPlay
  (CallFunction|AddSquishContext))

(event Collision|EventActorBeginOverlap
  (params (OtherActor :type Actor%20Object%20Reference)))

(event EventTick
  (params (DeltaSeconds :type Float%20%28single-precision%29)))

(fn ConstructionScript)

(fn AddSquishContext
  (Input|AddMappingContext (PlayerController|LocalPlayerSubsystems|GetEnhancedInputLocalPlayerSubsystem (Game|GetPlayerController 0)) "/Game/SquishySmash/Input/IMC_Squishy.IMC_Squishy" 1 "(bIgnoreAllPressedKeysUntilRelease=True,bForceImmediately=False,bNotifyUserSettings=False)"))

(fn OnSquishPressed
  (bind _returnvalue (Transformation|GetActorLocation))
  (bind _returnvalue_2 (Math|Vector|MakeVector 0.0 0.0 -45.0))
  (bind _returnvalue_3 (+ _returnvalue _returnvalue_2))
  (bind (_outhit _returnvalue_4) (Collision|LineTraceByChannel _returnvalue_3 (+ _returnvalue_3 (* (Math|Vector|GetForwardVector (Transformation|GetActorRotation)) (Math|Float|MakeLiteralFloat 4.5e+02))) "TraceTypeQuery1" true 0 "None"))
  (if _returnvalue_4
    (bind _asbp_squishy_friend (Utilities|Casting|CastToBP_SquishyFriend (.HitActor (Collision|BreakHitResult _outhit))))
    (Default|Squish _asbp_squishy_friend)))