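; BP_SquishyPlayerController is the Squishy Smash player controller that sets up Enhanced Input and passes the squish action to the character.
; One tick after BeginPlay it adds the default and mouse-look mapping contexts, plus IMC_Squishy at higher priority.
; IA_Squish calls RelaySquish, which prints a debug string, casts the controlled pawn to BP_SquishyCharacter and calls OnSquishPressed on it.
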(event Input|EnhancedActionEvents|EnhancedInputActionIA_Squish
  (params (ActionValue :type Boolean) (ElapsedSeconds :type Float%20%28double-precision%29) (TriggeredSeconds :type Float%20%28double-precision%29) (InputAction :type Input%20Action%20Object%20Reference :default "/Game/SquishySmash/Input/IA_Squish.IA_Squish"))
  (CallFunction|RelaySquish))

(event EventBeginPlay
  (bind _returnvalue (PlayerController|LocalPlayerSubsystems|GetEnhancedInputLocalPlayerSubsystem))
  (Utilities|FlowControl|DelayUntilNextTick)
  (Input|AddMappingContext _returnvalue "/Game/Input/IMC_Default.IMC_Default" 0 "(bIgnoreAllPressedKeysUntilRelease=True,bForceImmediately=False,bNotifyUserSettings=False)")
  (Input|AddMappingContext _returnvalue "/Game/Input/IMC_MouseLook.IMC_MouseLook" 0 "(bIgnoreAllPressedKeysUntilRelease=True,bForceImmediately=False,bNotifyUserSettings=False)")
  (Input|AddMappingContext _returnvalue "/Game/SquishySmash/Input/IMC_Squishy.IMC_Squishy" 1 "(bIgnoreAllPressedKeysUntilRelease=True,bForceImmediately=False,bNotifyUserSettings=False)"))

(event EventTick
  (params (DeltaSeconds :type Float%20%28single-precision%29)))

(fn ConstructionScript)

(fn RelaySquish
  (Development|PrintString "PC RELAY SQUISH")
  (bind _asbp_squishy_character (Utilities|Casting|CastToBP_SquishyCharacter (Pawn|GetControlledPawn)))
  (Default|OnSquishPressed _asbp_squishy_character))